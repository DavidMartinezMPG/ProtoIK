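; BP_Human is an interactable human that can be stabbed in the head with a sharp object, then ragdolls.
; On interact, it prints a debug string and, if the interaction's required tags include Object.Sharp, has the instigator's IKInteractionComponent move its upper socket to the head socket.
; When that socket arrives, the held actor attaches to the head keeping world transform, and mesh and capsule switch to simulated Ragdoll physics.
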(event `self.Interactable Component.OnInteract`
  (params (InstigatorComponent :type "InteractionComponent Object Reference") (InteractionTags :type "InteractionTags Structure"))
  (bind _returnvalue (`self.GetComponentByClass` (`ActorComponent.GetOwner` InstigatorComponent) "/Script/ProtoIK.IKInteractionComponent"))
  (`KismetSystemLibrary.PrintString` "INTERACTED")
  (if (`BlueprintGameplayTagLibrary.HasTag` InteractionTags_RequiredTags (struct :`TagName` "Object.Sharp") true)
    (`IKInteractionComponent.MoveUpperSocketTo` _returnvalue (`SceneComponent.GetSocketLocation` (`self.Mesh`) "head"))
    (add `IKInteractionComponent.OnUpperSocketReachedLocation` _returnvalue (delegate `OnUpperSocketReachedLocation_Event`))))

(event `OnUpperSocketReachedLocation_Event`
  (params (Location :type "Vector Structure"))
  (bind _mesh (`self.Mesh`))
  (bind _capsulecomponent (`self.CapsuleComponent`))
  (`self.K2_AttachToComponent` (`IKInteractionComponent.UpperSocketAttachedActor` (`self.GetComponentByClass` (`ActorComponent.GetOwner` (stale `self.Interactable Component.OnInteract` InstigatorComponent)) "/Script/ProtoIK.IKInteractionComponent")) (`self.Mesh`) "head" "KeepWorld" "KeepWorld" "KeepWorld" true)
  ;[1 1 1] Activate ragdoll
  (`PrimitiveComponent.SetSimulatePhysics` _mesh true)
  (`PrimitiveComponent.SetCollisionProfileName` _mesh "Ragdoll" true)
  (`PrimitiveComponent.SetSimulatePhysics` _capsulecomponent true)
  (`PrimitiveComponent.SetCollisionProfileName` _capsulecomponent "Ragdoll" true))

(fn `UserConstructionScript`)