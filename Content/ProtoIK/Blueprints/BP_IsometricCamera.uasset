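; BP_IsometricCamera is a camera actor that follows the first player's pawn at an isometric viewing angle.
; The construction script derives pitch from asin(1/√3), keeps the existing yaw and roll, and sets the camera to perspective rather than orthographic projection.
; On BeginPlay it caches the pawn, then each Tick lerps toward that pawn's location plus an offset, using delta time times a speed for smoothing.
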(event `self.ReceiveBeginPlay`
  (set `self.TargetActor` (`GameplayStatics.GetPlayerPawn` 0)))

(event `self.ReceiveTick`
  (params (DeltaSeconds :type "Float (single-precision)"))
  (bind _targetactor (`self.TargetActor`)
    (:`then`
      (`self.K2_SetActorLocation` (`KismetMathLibrary.VLerp` (`self.K2_GetActorLocation`) (+ (`self.K2_GetActorLocation` _targetactor) (`self.CameraOffset`)) (* DeltaSeconds (`self.Speed`)))))
    (:`else`)))

(fn `UserConstructionScript`
  (bind (_returnvalue_roll _returnvalue_pitch _returnvalue_yaw) (`KismetMathLibrary.BreakRotator` (`self.K2_GetActorRotation`)))
  (bind _result (`/Engine/EditorBlueprintResources/StandardMacros.NegateFloat` (`KismetMathLibrary.DegAsin` (/ 1.0 (`KismetMathLibrary.Sqrt` 3.0))))
    (:`  `
      (`self.K2_SetActorRotation` (`KismetMathLibrary.MakeRotator` _returnvalue_roll _result _returnvalue_yaw))
      (`CameraComponent.SetProjectionMode` (`self.CameraComponent`) "Perspective"))))